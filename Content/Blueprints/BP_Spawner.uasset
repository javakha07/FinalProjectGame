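; BP_Spawner spawns waves of BP_Enemy at random spawn positions, taking each wave's enemy count from the Waves map.
; Without an existing save, BeginPlay creates a BP_save holding the current wave and spawns immediately.
; An existing save is loaded, but the code restoring its level is disconnected.
; Tick searches for all enemies every frame and starts the next wave when none remain.
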(event `self.ReceiveBeginPlay`
  (`GameplayStatics.DoesSaveGameExist` "")
  (if true
    (bind _returnvalue (`GameplayStatics.LoadGameFromSlot` ""))
    (bind _asbp_save (cast `/Game/Blueprints/BP_save` _returnvalue))
    (else
      (bind _returnvalue_2 (`GameplayStatics.CreateSaveGameObject` "/Game/Blueprints/BP_save.BP_save_C"))
      (set `/Game/Blueprints/BP_save.Level` (`self.Current Wave`) _returnvalue_2)
      (`GameplayStatics.SaveGameToSlot` _returnvalue_2)
      (`self.Spawn Wave`))))

(event `Spawn Wave`
  (`/Engine/EditorBlueprintResources/StandardMacros.IncrementInt` (`self.Current Wave`)
    (:`  `
      (bind _values (`BlueprintMapLibrary.Map_Values` (`self.Waves`)))
      (for _ (range (+ (`|GetArrayItem` _values (- (`self.Current Wave`) 1)) 1))
        (`|SpawnActorFromClass` "/Game/Blueprints/BP_Enemy.BP_Enemy_C" (`KismetArrayLibrary.Array_Random` (`self.Spawn positions`)) "AdjustIfPossibleButAlwaysSpawn" "MultiplyWithRoot" null null)))))

(event `self.ReceiveTick`
  (params (DeltaSeconds :type "Float (single-precision)"))
  (bind _outactors (`GameplayStatics.GetAllActorsOfClass` "/Game/Blueprints/BP_Enemy.BP_Enemy_C"))
  (if (== (`KismetArrayLibrary.Array_Length` _outactors) 0)
    (`self.Spawn Wave`)))

(fn `UserConstructionScript`)