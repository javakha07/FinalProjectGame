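; Player character Blueprint that handles movement, camera look, a shove melee attack and health.
; BeginPlay adds the Enhanced Input mapping context and creates health and HUD widgets, while input events drive control-rotation-relative movement and look.
; The shove montage locks re-attacking until completion, and its notify runs a sphere trace from AttackRange to damage pawns.
; Incoming damage lowers Health and flashes the HUD; at zero, input is disabled and the mesh ragdolls.
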(event `self.ReceiveBeginPlay`
  ;[1 1 1] Input
  (`EnhancedInputSubsystemInterface.AddMappingContext` (pcsubsystem `EnhancedInputLocalPlayerSubsystem` (`GameplayStatics.GetPlayerController` 0)) "/Game/Inputs/IMC_PlayerInput.IMC_PlayerInput" 0 (struct))
  (bind _returnvalue (`|CreateWidget` "/Game/UI/WB_Health.WB_Health_C"))
  (`UserWidget.AddToViewport` _returnvalue 0)
  (bind _returnvalue_2 (`|CreateWidget` "/Game/UI/WB_HUD.WB_HUD_C"))
  (bind _output_get (set `self.HUD` _returnvalue_2))
  (`UserWidget.AddToViewport` _output_get 0))

(event `EnhancedInput|/Game/Inputs/IA_Movement`
  (params (ActionValue :type "Vector2D Structure") (ElapsedSeconds :type "Float (double-precision)") (TriggeredSeconds :type "Float (double-precision)") (InputAction :type "InputAction Object Reference" :default "/Game/Inputs/IA_Movement.IA_Movement"))
  (bind (_returnvalue_roll _returnvalue_pitch _returnvalue_yaw) (`KismetMathLibrary.BreakRotator` (`self.GetControlRotation`)))
  (bind (_returnvalue_roll_2 _returnvalue_pitch_2 _returnvalue_yaw_2) (`KismetMathLibrary.BreakRotator` (`self.GetControlRotation`)))
  ;[1 1 1] Movement
  (:`Triggered`
    (`self.AddMovementInput` (`KismetMathLibrary.GetRightVector` (`KismetMathLibrary.MakeRotator` _returnvalue_roll_2 0.0 _returnvalue_yaw_2)) ActionValue_X)
    (`self.AddMovementInput` (`KismetMathLibrary.GetForwardVector` (`KismetMathLibrary.MakeRotator` _returnvalue_roll 0.0 _returnvalue_yaw)) ActionValue_Y)))

(event `EnhancedInput|/Game/Inputs/IA_CAM`
  (params (ActionValue :type "Vector2D Structure") (ElapsedSeconds :type "Float (double-precision)") (TriggeredSeconds :type "Float (double-precision)") (InputAction :type "InputAction Object Reference" :default "/Game/Inputs/IA_CAM.IA_CAM"))
  ;[1 1 1] Movement
  (:`Triggered`
    (`self.AddControllerYawInput` ActionValue_X)
    (`self.AddControllerPitchInput` (* ActionValue_Y -1.0))))

(event `EnhancedInput|/Game/Inputs/IA_shove`
  (params (ActionValue :type Boolean) (ElapsedSeconds :type "Float (double-precision)") (TriggeredSeconds :type "Float (double-precision)") (InputAction :type "InputAction Object Reference" :default "/Game/Inputs/IA_shove.IA_shove"))
  (bind _attackrange (`self.AttackRange`))
  (bind _returnvalue (`SceneComponent.K2_GetComponentLocation` _attackrange))
  ;[1 1 1] Attack
  (:`Started`
    (if (`self.Can Attack`)
      (`|PlayMontage` (`self.Mesh`) "/Game/Characters/Mannequins/Animations/Manny/shove_Montage.shove_Montage"
        (:`then`
          (set `self.Can Attack` false))
        (:`OnCompleted`
          (set `self.Can Attack` true))
        (:`OnNotifyBegin`
          (bind (_outhit _returnvalue_2) (`KismetSystemLibrary.SphereTraceSingleForObjects` :`Start` _returnvalue :`End` (+ _returnvalue (* (`SceneComponent.GetForwardVector` _attackrange) 150.0)) :`Radius` 30.0 :`ObjectTypes` (`|MakeArray` "ObjectTypeQuery3" :!type "EObjectTypeQuery Enum") :`DrawDebugType` "ForDuration"))
          (if _returnvalue_2
            (`GameplayStatics.ApplyDamage` (`.HitActor` (`GameplayStatics.BreakHitResult` _outhit)) 10.0)))))))

(event `self.ReceiveAnyDamage`
  (params (Damage :type "Float (single-precision)") (DamageType :type "DamageType Object Reference") (InstigatedBy :type "Controller Object Reference") (DamageCauser :type "Actor Object Reference"))
  ;[1 1 1] Take Damage
  (set `self.Health` (- (`self.Health`) Damage))
  (`/Game/UI/WB_HUD.Damage Screen` (`self.HUD`))
  (if (<= (`self.Health`) 0.0)
    (`self.DisableInput` null)
    (`PrimitiveComponent.SetSimulatePhysics` (`self.Mesh`) true)
    (else
      (`KismetSystemLibrary.PrintString` (`KismetStringLibrary.Conv_DoubleToString` (`self.Health`))))))

(fn `UserConstructionScript`)